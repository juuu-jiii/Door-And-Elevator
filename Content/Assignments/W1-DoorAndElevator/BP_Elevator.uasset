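; BP_Elevator is a player-controlled elevator that moves between a ground and a raised position.
; A box overlap with ThirdPersonCharacter enables actor input, letting MoveElevatorUp and MoveElevatorDown play or reverse one timeline.
; The timeline sets the scene root's absolute world Z, carrying the collider along but relying on a hardcoded start height.
; IsMoving and OnGround flags block presses mid-travel or toward the current position.
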(event OnComponentBeginOverlap(Box)
  (params (OverlappedComponent :type Primitive%20Component%20Object%20Reference) (OtherActor :type Actor%20Object%20Reference) (OtherComp :type Primitive%20Component%20Object%20Reference) (OtherBodyIndex :type Integer) (bFromSweep :type Boolean) (SweepResult :type Hit%20Result%20Structure%20%28by%20ref%29))
  ;[1 1 1] Allow elevator to listen for keyboard input when player collides with it.
  (Utilities|Casting|CastToThirdPersonCharacter OtherActor) ; Cast the Actor colliding with the box to ThirdPersonCharacter
  (Input|EnableInput (Game|GetPlayerController 0)) ; Enable input on THIS Actor
)

(event OnComponentEndOverlap(Box)
  (params (OverlappedComponent :type Primitive%20Component%20Object%20Reference) (OtherActor :type Actor%20Object%20Reference) (OtherComp :type Primitive%20Component%20Object%20Reference) (OtherBodyIndex :type Integer))
  ;[1 1 1] Disable keyboard input listening when player no longer overlaps with elevator
  (Utilities|Casting|CastToThirdPersonCharacter OtherActor) ; Cast the Actor colliding with the box to ThirdPersonCharacter
  (Input|DisableInput (Game|GetPlayerController 0)) ; Disable input on THIS Actor
)

(event EventBeginPlay
  (Variables|Default|SetIsMoving false)
  (Variables|Default|SetOnGround true))

(event Collision|EventActorBeginOverlap
  (params (OtherActor :type Actor%20Object%20Reference)))

(event EventTick
  (params (DeltaSeconds :type Float%20%28single-precision%29)))

(event Input|ActionEvents|InputActionMoveElevatorUp
  (params (Key :type Key%20Structure :default "None"))
  (bind _returnvalue (Transformation|GetActorLocation))
  ;[1 1 1] Move elevator up.
  (:Pressed
    (if (and (not (Variables|Default|GetIsMoving)) (Variables|Default|GetOnGround))
      (Variables|Default|SetIsMoving true) ; Elevator is moving
      (Variables|Default|SetOnGround false) ; Elevator is in the air
      ;[1 1 1] Elevator movement and animation
      (bind _elevatorup_float (Timeline|ElevatorUp PlayFromStart) ; Adjust timing and smoothness of elevator movement animation\nFloat = final Z-position (note that initial Z-position was hardcoded)\nVector = NONE
        (:Update
          (Transformation|SetWorldLocation (Variables|Default|GetDefaultSceneRoot) (Math|Vector|MakeVector (.x _returnvalue) (.y _returnvalue) _elevatorup_float) false false) ; Move the scene root up/down
        )
        (:Finished
          (Variables|Default|SetIsMoving false) ; Elevator is stationary
        )))))

(event Input|ActionEvents|InputActionMoveElevatorDown
  (params (Key :type Key%20Structure :default "None"))
  (bind _returnvalue (Transformation|GetActorLocation))
  ;[1 1 1] Move elevator down.
  (:Pressed
    (if (and (not (Variables|Default|GetIsMoving)) (not (Variables|Default|GetOnGround)))
      (Variables|Default|SetIsMoving true) ; Elevator is moving
      (Variables|Default|SetOnGround true) ; Elevator is on the ground
      ;[1 1 1] Elevator movement and animation
      (bind _elevatorup_float (Timeline|ElevatorUp ReverseFromEnd) ; Adjust timing and smoothness of elevator movement animation\nFloat = final Z-position (note that initial Z-position was hardcoded)\nVector = NONE
        (:Update
          (Transformation|SetWorldLocation (Variables|Default|GetDefaultSceneRoot) (Math|Vector|MakeVector (.x _returnvalue) (.y _returnvalue) _elevatorup_float) false false) ; Move the scene root up/down
        )
        (:Finished
          (Variables|Default|SetIsMoving false) ; Elevator is stationary
        )))))

(fn ConstructionScript)

(fn TestFunction)